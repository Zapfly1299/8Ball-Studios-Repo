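; Construction-script prop generator that lays out a row of book static meshes in the editor.
; Each loop step up to AmountOfBooks randomly picks one of three mesh branches, then shifts the Location transform along negative X by that branch's spacing.
; Each branch test re-rolls the random number, so odds are uneven and some steps add no book.
; Either Refresh or Refresh1 triggers the build; the event graph is unused.
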(fn `UserConstructionScript`
  (bind _returnvalue (`KismetMathLibrary.RandomIntegerInRange` 0 2))
  (bind _location (`self.Location`))
  (bind _location_2 (`self.Location`))
  (bind _location_3 (`self.Location`))
  (if (`self.Refresh`)
    (for _ (range (+ (`self.Amount Of Books`) 1)) :!label _label
      (if (== _returnvalue 0)
        (`AddComponent|NODE_AddStaticMeshComponent-3` :`RelativeTransform` (`self.Location`))
        (set `self.Location` (`KismetMathLibrary.MakeTransform` (`KismetMathLibrary.MakeVector` (- (.x (.location _location_2)) 3.0) (.y (.location _location_2)) (.z (.location _location_2))) (.rotation _location_2) (.scale _location_2)))
        (elif (== _returnvalue 1)
          (`AddComponent|NODE_AddStaticMeshComponent-4` :`RelativeTransform` (`self.Location`))
          (set `self.Location` (`KismetMathLibrary.MakeTransform` (`KismetMathLibrary.MakeVector` (- (.x (.location _location_3)) 3.1) (.y (.location _location_3)) (.z (.location _location_3))) (.rotation _location_3) (.scale _location_3)))
          (elif (== _returnvalue 2)
            (`AddComponent|NODE_AddStaticMeshComponent-5` :`RelativeTransform` (`self.Location`))
            (set `self.Location` (`KismetMathLibrary.MakeTransform` (`KismetMathLibrary.MakeVector` (- (.x (.location _location)) 5.0) (.y (.location _location)) (.z (.location _location))) (.rotation _location) (.scale _location)))))))
    (elif (`self.Refresh_1`)
      (set `self.Refresh` false)
      (set `self.Refresh` false)
      (goto _label))))