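; Procedural book-row prop that fills a line with randomly picked static mesh books in the construction script.
; It rebuilds when the Refresh toggle is set, which then clears itself, or on every construction run with AlwaysUpdate.
; Each loop pass re-rolls through six branches, so it may place nothing.
; Placed books get a random or fixed Y push, then step the Location cursor along negative X by a per-branch width.
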(fn `UserConstructionScript`
  (bind _returnvalue (`KismetMathLibrary.RandomIntegerInRange` 0 5))
  (bind _location (`self.Location`))
  (bind _location_2 (`self.Location`))
  (bind _location_3 (`self.Location`))
  (bind _location_4 (`self.Location`))
  (bind _location_5 (`self.Location`))
  (bind _location_6 (`self.Location`))
  (bind _location_7 (`self.Location`))
  (bind _location_8 (`self.Location`))
  (bind _location_9 (`self.Location`))
  (bind _location_10 (`self.Location`))
  (bind _location_11 (`self.Location`))
  (bind _location_12 (`self.Location`))
  (bind _returnvalue_2 (`KismetMathLibrary.RandomFloatInRange` 0.0 (`self.PushInOutRange`)))
  (if (`self.Refresh`)
    (set `self.Refresh` false)
    (for _ (range (+ (`self.Amount Of Books`) 1)) :!label _label
      (if (== _returnvalue 0)
        (`AddComponent|NODE_AddStaticMeshComponent-3` :`RelativeTransform` (`KismetMathLibrary.MakeTransform` (`KismetMathLibrary.MakeVector` (.x (.location _location_10)) (- (.y (.location _location_10)) _returnvalue_2) (.z (.location _location_10)))))
        (set `self.Location` (`KismetMathLibrary.MakeTransform` (`KismetMathLibrary.MakeVector` (- (.x (.location _location_10)) 3.0) (.y (.location _location_3)) (.z (.location _location_3))) (.rotation _location_3) (.scale _location_3)))
        (elif (== _returnvalue 1)
          (`AddComponent|NODE_AddStaticMeshComponent-4` :`RelativeTransform` (`KismetMathLibrary.MakeTransform` (`KismetMathLibrary.MakeVector` (.x (.location _location_11)) (- (.y (.location _location_11)) _returnvalue_2) (.z (.location _location_11)))))
          (set `self.Location` (`KismetMathLibrary.MakeTransform` (`KismetMathLibrary.MakeVector` (- (.x (.location _location_11)) 3.1) (.y (.location _location_4)) (.z (.location _location_4))) (.rotation _location_4) (.scale _location_4)))
          (elif (== _returnvalue 2)
            (`AddComponent|NODE_AddStaticMeshComponent-5` :`RelativeTransform` (`KismetMathLibrary.MakeTransform` (`KismetMathLibrary.MakeVector` (.x (.location _location)) (- (.y (.location _location)) _returnvalue_2) (.z (.location _location)))))
            (set `self.Location` (`KismetMathLibrary.MakeTransform` (`KismetMathLibrary.MakeVector` (- (.x (.location _location)) 5.0) (.y (.location _location_5)) (.z (.location _location_5))) (.rotation _location_5) (.scale _location_5)))
            (elif (== _returnvalue 3)
              (`AddComponent|NODE_AddStaticMeshComponent-6` :`RelativeTransform` (`KismetMathLibrary.MakeTransform` (`KismetMathLibrary.MakeVector` (.x (.location _location_6)) (- (.y (.location _location_6)) _returnvalue_2) (.z (.location _location_6)))))
              (set `self.Location` (`KismetMathLibrary.MakeTransform` (`KismetMathLibrary.MakeVector` (- (.x (.location _location_6)) 2.7) (.y (.location _location_7)) (.z (.location _location_7))) (.rotation _location_7) (.scale _location_7)))
              (elif (== _returnvalue 4)
                (`AddComponent|NODE_AddStaticMeshComponent-7` :`RelativeTransform` (`KismetMathLibrary.MakeTransform` (`KismetMathLibrary.MakeVector` (.x (.location _location_8)) (- (.y (.location _location_8)) 1.0) (.z (.location _location_8)))))
                (set `self.Location` (`KismetMathLibrary.MakeTransform` (`KismetMathLibrary.MakeVector` (- (.x (.location _location_8)) 5.4) (.y (.location _location_9)) (.z (.location _location_9))) (.rotation _location_9) (.scale _location_9)))
                (elif (== _returnvalue 5)
                  (`AddComponent|NODE_AddStaticMeshComponent-8` :`RelativeTransform` (`KismetMathLibrary.MakeTransform` (`KismetMathLibrary.MakeVector` (.x (.location _location_12)) (- (.y (.location _location_12)) 1.0) (.z (.location _location_12)))))
                  (set `self.Location` (`KismetMathLibrary.MakeTransform` (`KismetMathLibrary.MakeVector` (- (.x (.location _location_12)) 4.9) (.y (.location _location_2)) (.z (.location _location_2))) (.rotation _location_2) (.scale _location_2))))))))))
    (elif (`self.Always Update`)
      (goto _label))))