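; Teleporter actor that moves actors entering its box to the spawn point of a linked teleporter.
; Begin overlap adds the actor to an array and, if teleporting is allowed, moves every tracked actor; end overlap removes it.
; Each jump plays a timeline scaling the ray on both teleporters.
; Only the destination's SafetyCheck runs, blocking it for a cooldown to prevent an immediate return.
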(event `SafetyCheck`
  (set `self.CanTeleport` false)
  (`KismetSystemLibrary.Delay` (`self.TeleportCooldown`))
  (set `self.CanTeleport` true))

(event `Teleport`
  ;[1 0.3137 0.8667] Handles the animation (or particles) of teleporter and puts it onto a cooldown.
  ;;[1 0.3137 0.8667] Sets scale of teleport ray, this can be changed or swapped for particle effects.
  (bind (_direction _alpha) (`Timeline|MoveTeleportRay` :!label _label)
    (:`Update`
      (`SceneComponent.SetRelativeScale3D` (`self.TeleportRay`) (`KismetMathLibrary.VLerp` (`self.RayStartScale`) (`self.RayEndScale`) _alpha)))))

(event `ReverseIncoming`
  ;[1 0.3137 0.8667] Handles the animation (or particles) of teleporter and puts it onto a cooldown.
  ;;[1 0.3137 0.8667] Sets scale of teleport ray, this can be changed or swapped for particle effects.
  (goto _label :!via `Reverse`))

(event `self.Box.OnComponentBeginOverlap`
  (params (OverlappedComponent :type "PrimitiveComponent Object Reference") (OtherActor :type "Actor Object Reference") (OtherComp :type "PrimitiveComponent Object Reference") (OtherBodyIndex :type Integer) (bFromSweep :type Boolean) (SweepResult :type "HitResult Structure (by ref)"))
  ;[1 0.3137 0.8667] Checks overlap and does check to see if overlapped actor is still inside collision before teleporting. This prevents actors running over and instantly being teleported.
  (`KismetArrayLibrary.Array_AddUnique` (`self.OverlappedActors`) OtherActor)
  (if (`self.CanTeleport`)
    (for _array_element (`self.OverlappedActors`)
      (`/Engine/EditorBlueprintResources/StandardMacros.IsValid` _array_element
        (:`Is Valid`
          (`self.Teleport`)
          (`self.SafetyCheck` (`self.LinkedTeleporter`))
          (`self.Teleport` (`self.LinkedTeleporter`))
          (`self.K2_SetActorLocation` _array_element (`SceneComponent.K2_GetComponentLocation` (`/Game/Blueprints/KyleStuff/BP_TestTeleporter.Spawn Point` (`self.LinkedTeleporter`))) false false))))))

(event `self.Box.OnComponentEndOverlap`
  (params (OverlappedComponent :type "PrimitiveComponent Object Reference") (OtherActor :type "Actor Object Reference") (OtherComp :type "PrimitiveComponent Object Reference") (OtherBodyIndex :type Integer))
  ;[1 0.3137 0.8667] When the actor which initially overlapped leaves the collision box, the actor gets emptied so they don't get teleported. This MAY cause issues in the future since it can only handle one actor at a time. This may need to be worked on with arrays.
  (`KismetArrayLibrary.Array_RemoveItem` (`self.OverlappedActors`) OtherActor))

(fn `UserConstructionScript`)