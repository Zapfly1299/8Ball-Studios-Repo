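; Double-door entrance Blueprint that swings left and right doors open and closed.
; BeginPlay snaps both doors to their start rotations, which serve as the open pose.
; CloseEntrance and OpenEntrance each drive one timeline per door, lerping relative rotation between start and end rotators.
; Both events also call SetCollisions, passing false when closing and true when opening.
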(event `self.ReceiveBeginPlay`
  (`SceneComponent.K2_SetRelativeRotation` (`self.Door_Right`) (`self.StartRightRot`) false false)
  (`SceneComponent.K2_SetRelativeRotation` (`self.Door_Left`) (`self.StartLeftRot`) false false))

(event `self.CloseEntrance`
  ;[1 0.3137 0.8667] Closes doors when the event is called.
  (`self.SetCollisions` false)
  (`|ExecutionSequence`
    (:`then_0`
      (bind (_direction _alpha) (`Timeline|Timeline_0`)
        (:`Update`
          (`SceneComponent.K2_SetRelativeRotation` (`self.Door_Left`) (`KismetMathLibrary.RLerp` (`self.StartLeftRot`) (`self.EndLeftRot`) _alpha) false false))
        (:`Finished`)))
    (:`then_1`
      (bind (_direction_2 _alpha_2) (`Timeline|Timeline_1`)
        (:`Update`
          (`SceneComponent.K2_SetRelativeRotation` (`self.Door_Right`) (`KismetMathLibrary.RLerp` (`self.StartRightRot`) (`self.EndRightRot`) _alpha_2) false false))))))

(event `self.OpenEntrance`
  ;[1 0.3137 0.8667] Opens the doors when the event is called.
  (`self.SetCollisions` true)
  (`|ExecutionSequence`
    (:`then_0`
      (bind (_direction _alpha) (`Timeline|Timeline_2` :!via `PlayFromStart`)
        (:`Update`
          (`SceneComponent.K2_SetRelativeRotation` (`self.Door_Left`) (`KismetMathLibrary.RLerp` (`self.EndLeftRot`) (`self.StartLeftRot`) _alpha) false false))))
    (:`then_1`
      (bind (_direction_2 _alpha_2) (`Timeline|Timeline_3` :!via `PlayFromStart`)
        (:`Update`
          (`SceneComponent.K2_SetRelativeRotation` (`self.Door_Right`) (`KismetMathLibrary.RLerp` (`self.EndRightRot`) (`self.StartRightRot`) _alpha_2) false false))))))

(fn `UserConstructionScript`
  (`parent.UserConstructionScript`))