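; BP_TomeCollectible is a pickup that grants the first-person player tome charge on touch.
; It caches the player pawn as a FirstPersonCharacter reference on BeginPlay.
; When its Sphere overlaps an actor of exactly that class, a DoOnce gate lets it add a fixed charge to the cached player and destroy itself.
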(event `self.ReceiveBeginPlay`
  (bind _asfirst_person_character (cast `/Game/Blueprints/FirstPersonCharacter` (`GameplayStatics.GetPlayerPawn` 0)))
  (set `self.PlayerRef` _asfirst_person_character))

(event `self.Sphere.OnComponentBeginOverlap`
  (params (OverlappedComponent :type "PrimitiveComponent Object Reference") (OtherActor :type "Actor Object Reference") (OtherComp :type "PrimitiveComponent Object Reference") (OtherBodyIndex :type Integer) (bFromSweep :type Boolean) (SweepResult :type "HitResult Structure (by ref)"))
  (if (== (`GameplayStatics.GetObjectClass` OtherActor) "/Game/Blueprints/FirstPersonCharacter.FirstPersonCharacter_C")
    (`/Engine/EditorBlueprintResources/StandardMacros.DoOnce` false
      (:`Completed`
        (`/Game/Blueprints/FirstPersonCharacter.AddTomeCharge` (`self.PlayerRef`) 2.0)
        (`self.K2_DestroyActor`)))))

(fn `UserConstructionScript`)