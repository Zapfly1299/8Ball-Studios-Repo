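; BP_WeaponCrate is a crate that adds a weapon class to the player's Weapons array on Interact.
; Box overlap with FirstPersonCharacter enables input and opens a gate, and end overlap reverses both.
; In random mode, the WeaponChecker macro strips already-owned weapons before a shuffle picks one; otherwise it gives WeaponToSpawn.
; A successful grant destroys the Box component, leaving the actor itself in place.
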(event `self.ReceiveBeginPlay`
  ;[1 0.3137 0.8667] Gets player reference
  (bind _asfirst_person_character (cast `/Game/Blueprints/FirstPersonCharacter` (`GameplayStatics.GetPlayerPawn` 0)))
  (set `self.PlayerRef` _asfirst_person_character))

(event `InputAction|Interact`
  (params (Key :type "Key Structure"))
  (bind _output (`|GetArrayItem` (`self.Weapons`)))
  ;[1 0.3137 0.8667] Allows player to interact, stops enemies being able to mess with interaction.
  (:`Pressed`
    (`/Engine/EditorBlueprintResources/StandardMacros.Gate` true :!label _label
      (:`Exit`
        (if (`self.IsRandom?`)
          (for _array_element (`self.Weapons`)
            (for _array_element_2 (`/Game/Blueprints/FirstPersonCharacter.Weapons` (`self.PlayerRef`))
              (if (== _array_element _array_element_2)
                (`KismetArrayLibrary.Array_RemoveItem` (`self.Weapons`) _array_element_2))))
          ;[1 0.3137 0.8667] Gets a random weapon out of array and adds it to player.
          (`KismetArrayLibrary.Array_Shuffle` (`self.Weapons`))
          (if (`KismetSystemLibrary.IsValidClass` _output)
            (`KismetArrayLibrary.Array_Add` (`/Game/Blueprints/FirstPersonCharacter.Weapons` (`self.PlayerRef`)) _output)
            (`ActorComponent.K2_DestroyComponent` (`self.Box`)))
          (else
            (`KismetArrayLibrary.Array_Add` (`/Game/Blueprints/FirstPersonCharacter.Weapons` (`self.PlayerRef`)) (`self.WeaponToSpawn`))
            (`ActorComponent.K2_DestroyComponent` (`self.Box`))))))))

(event `self.Box.OnComponentBeginOverlap`
  (params (OverlappedComponent :type "PrimitiveComponent Object Reference") (OtherActor :type "Actor Object Reference") (OtherComp :type "PrimitiveComponent Object Reference") (OtherBodyIndex :type Integer) (bFromSweep :type Boolean) (SweepResult :type "HitResult Structure (by ref)"))
  ;[1 0.3137 0.8667] Allows player to interact, stops enemies being able to mess with interaction.
  (if (== (`GameplayStatics.GetObjectClass` OtherActor) "/Game/Blueprints/FirstPersonCharacter.FirstPersonCharacter_C")
    (`self.EnableInput` (`GameplayStatics.GetPlayerController` 0))
    (goto _label :!via `Open`)))

(event `self.Box.OnComponentEndOverlap`
  (params (OverlappedComponent :type "PrimitiveComponent Object Reference") (OtherActor :type "Actor Object Reference") (OtherComp :type "PrimitiveComponent Object Reference") (OtherBodyIndex :type Integer))
  ;[1 0.3137 0.8667] Allows player to interact, stops enemies being able to mess with interaction.
  (if (== (`GameplayStatics.GetObjectClass` OtherActor) "/Game/Blueprints/FirstPersonCharacter.FirstPersonCharacter_C")
    (`self.DisableInput` (`GameplayStatics.GetPlayerController` 0))
    (goto _label :!via `Close`)))

(fn `UserConstructionScript`)