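; Room manager that runs a combat encounter: player overlap closes the doors, removes the trigger and starts the waves if enabled.
; Up to three configured waves show spawn decals, then after a delay spawn AI enemies that receive a manager reference.
; Enemy deaths trigger a debounced "Enemy" tag count, starting the next wave or finishing the room.
; Finishing opens doors, detonates mines, awards a random weapon and optionally spawns an item stand or shows the end screen.
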(event `self.ReceiveBeginPlay`
  (bind _asfirst_person_character (cast `/Game/Blueprints/FirstPersonCharacter` (`GameplayStatics.GetPlayerPawn` 0)))
  (set `self.PlayerRef` _asfirst_person_character))

(event `self.Cube.OnComponentBeginOverlap`
  (params (OverlappedComponent :type "PrimitiveComponent Object Reference") (OtherActor :type "Actor Object Reference") (OtherComp :type "PrimitiveComponent Object Reference") (OtherBodyIndex :type Integer) (bFromSweep :type Boolean) (SweepResult :type "HitResult Structure (by ref)"))
  ;[1 0.3137 0.8667] This blueprint will handle most of the interactions within each room. Will act as a communicator between BPs
  ;;[1 0.3137 0.8667] When player overlaps, causes doors to close and destroys box collider to prevent issues.
  (if (== (`GameplayStatics.GetObjectClass` OtherActor) "/Game/Blueprints/FirstPersonCharacter.FirstPersonCharacter_C")
    (`|ExecutionSequence`
      (:`then_0`
        (if (`self.CanSpawn?`)
          (`self.NewWave`)
          (`KismetSystemLibrary.Delay` (`self.WaveDelay`))
          (`self.StartSpawning`)))
      (:`then_1`
        (for _array_element (`self.Door`)
          (`/Game/Blueprints/KyleStuff/BP_BaseDoor.CloseEntrance` _array_element))
        (`ActorComponent.K2_DestroyComponent` (`self.Cube`))))))

(event `StartSpawning`
  ;[1 0.3137 0.8667] This blueprint will handle most of the interactions within each room. Will act as a communicator between BPs
  ;;[1 0.3137 0.8667] Spawns enemies using the spawner information struct which can be set in viewport.
  (for _array_element (`self.SpawnInformation`)
    (`self.SpawnEnemies` _array_element)))

(event `EnemyDied`
  ;[1 0.3137 0.8667] When enemy dies, checks to see if there's no enemies left in the room
  (`KismetSystemLibrary.RetriggerableDelay` 1.0)
  (bind _outactors (`GameplayStatics.GetAllActorsWithTag` "Enemy"))
  (if (== (`KismetArrayLibrary.Array_Length` _outactors) 0)
    ;[1 0.3137 0.8667] Checks if waves are complete and if not, starts the next wave. If complete, calls room finished.
    (if (`self.WavesComplete`)
      (`self.Room Finished`)
      (else
        (`self.NewWave`)
        (`KismetSystemLibrary.Delay` (`self.WaveDelay`))
        (`self.StartSpawning`)))))

(event `Room Finished`
  ;[1 0.3137 0.8667] Handles all the end of room logic
  ;;[1 0.3137 0.8667] Reopens all the doors when the room is finished
  (for _array_element (`self.Door`)
    (`/Game/Blueprints/KyleStuff/BP_BaseDoor.OpenEntrance` _array_element)
    ;;[1 0.3137 0.8667] Destroys all mines when room is completed
    (bind _outactors (`GameplayStatics.GetAllActorsOfClass` "/Game/AI/BP_Mine.BP_Mine_C"))
    (for _array_element_2 _outactors
      (`/Game/AI/BP_Mine.Detonate` _array_element_2))
    (`|ExecutionSequence`
      (:`then_0`
        ;;[1 0.3137 0.8667] When room is finished and it is the final room, it will bring up the win screen.
        (if (`self.FinalRoom?`)
          (`KismetSystemLibrary.Delay` 2.0)
          (`GameplayStatics.SetGamePaused` true)
          (set `PlayerController.bShowMouseCursor` true (`GameplayStatics.GetPlayerController` 0))
          (bind _returnvalue (`|CreateWidget` "/Game/Widgets/WBP_EndScreen.WBP_EndScreen_C"))
          (`UserWidget.AddToViewport` _returnvalue 0)
          (`WidgetBlueprintLibrary.SetInputMode_UIOnlyEx` (`GameplayStatics.GetPlayerController` 0) _returnvalue)))
      (:`then_1`
        ;;[1 0.3137 0.8667] If set true, spawns an item stand on the location of the item spawn.
        (if (`self.SpawnItem?`)
          (`|SpawnActorFromClass` "/Game/Blueprints/ItemRoom/BP_ItemStand.BP_ItemStand_C" (`self.GetTransform` (`self.ItemSpawn`)) "Undefined" "OverrideRootScale" null null)))
      (:`then_2`
        (bind _keys (`BlueprintMapLibrary.Map_Keys` (`self.Weapons`)))
        (for _array_element_3 _keys
          (for _array_element_4 (`/Game/Blueprints/FirstPersonCharacter.Weapons` (`self.PlayerRef`))
            (if (== _array_element_3 _array_element_4)
              (bind _keys_2 (`BlueprintMapLibrary.Map_Keys` (`self.Weapons`)))
              (`KismetArrayLibrary.Array_RemoveItem` _keys_2 _array_element_4))))
        (bind _keys_3 (`BlueprintMapLibrary.Map_Keys` (`self.Weapons`)))
        (bind _output (`|GetArrayItem` _keys_3 (`self.RandomInt` _keys_3)))
        (if (`KismetSystemLibrary.IsValidClass` _output)
          (`KismetArrayLibrary.Array_Add` (`/Game/Blueprints/FirstPersonCharacter.Weapons` (`self.PlayerRef`)) _output)
          (`/Game/Widgets/WBP_PlayerHUD.NewWeapon` (`/Game/Blueprints/FirstPersonCharacter.HUDRef` (`self.PlayerRef`)) (`self.Weapons`) (`self.RandomWeaponInt`)))))))

(fn `CheckWaveCount`
  (params (Wave :type Integer))
  (returns (`WavesComplete?` :type Boolean))
  (return (== Wave (`self.WavesAmount`))))

(fn `NewWave`
  ;[1 0.3137 0.8667] Sets up spawn information and checks if it has reached final wave
  (bind _result (`/Engine/EditorBlueprintResources/StandardMacros.IncrementInt` (`self.CurrentWave`))
    (:`  `
      (switch `int` _result
        (:`1`
          (set `self.SpawnInformation` (`self.Wave1`)))
        (:`2`
          (set `self.SpawnInformation` (`self.Wave2`)))
        (:`3`
          (set `self.SpawnInformation` (`self.Wave3`))))
      (set `self.WavesComplete` (`self.CheckWaveCount` (`self.CurrentWave`)))
      (for _array_element (`self.SpawnInformation`)
        (`/Game/Blueprints/KyleStuff/BP_SpawnPoint.SpawnDecal` (`.SpawnPoint_10_9D5908354404A1AF3DFD7FB1B58C568B` (break `/Game/Blueprints/KyleStuff/S_SpawnInfo` _array_element)))))))

(fn `RandomInt`
  (params (TargetArray :type "Array of /Game/Blueprints/Weapons/BP_GunBase Class Reference (by ref)"))
  (returns (Output_Get :type Integer))
  (bind _output_get (set `self.RandomWeaponInt` (`KismetMathLibrary.RandomIntegerInRange` 0 (- (`KismetArrayLibrary.Array_Length` TargetArray) 1))))
  (return _output_get))

(fn `SpawnEnemies`
  (params (`Spawn Information` :type "/Game/Blueprints/KyleStuff/S_SpawnInfo Structure"))
  (bind (_enemypawn _behaviourtree _spawnpoint) (break `/Game/Blueprints/KyleStuff/S_SpawnInfo` `Spawn Information`))
  (bind _arrow (`/Game/Blueprints/KyleStuff/BP_SpawnPoint.Arrow` _spawnpoint))
  ;[1 0.3137 0.8667] Takes the struct information and inputs it into the spawn AI from class. Also sends the reference to the manager to the enemies so they can interact with the room manager.
  (bind _returnvalue (`AIBlueprintHelperLibrary.SpawnAIFromClass` _enemypawn _behaviourtree (`SceneComponent.K2_GetComponentLocation` _arrow) (`SceneComponent.K2_GetComponentRotation` _arrow) false null))
  (message `/Game/Blueprints/KyleStuff/BPI_Manager.SendManagerRef` _returnvalue self))

(fn `UserConstructionScript`)