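; BP_Collectible is a pickup actor whose kind is set by a CollectibleType enum, with Health and two example types.
; On BeginPlay it switches on the enum and calls SetUp to give CollectibleMesh the matching static mesh.
; Box overlap checks that the other actor's class is exactly FirstPersonCharacter, then switches on the type, but no pickup effects are implemented yet.
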(event `self.ReceiveBeginPlay`
  ;[1 0.3137 0.8667] This will decide the mesh of the collectible when it is dropped. The enum variable can be changed when actor is spawned by blueprint or it can be changed when dragged into worldspace.
  (switch `/Game/Blueprints/KyleStuff/Enum_Collectibles` (`self.CollectibleType`)
    (:`NewEnumerator0`
      (`self.SetUp` "/Game/Geometry/Meshes/1M_Cube.1M_Cube"))
    (:`NewEnumerator1`
      (`self.SetUp` "/Game/Blueprints/ItemRoom/xD.xD"))
    (:`NewEnumerator2`
      (`self.SetUp` "/Game/Props/Weapons/Knife_Blockout.Knife_Blockout"))))

(event `self.Box.OnComponentBeginOverlap`
  (params (OverlappedComponent :type "PrimitiveComponent Object Reference") (OtherActor :type "Actor Object Reference") (OtherComp :type "PrimitiveComponent Object Reference") (OtherBodyIndex :type Integer) (bFromSweep :type Boolean) (SweepResult :type "HitResult Structure (by ref)"))
  ;[1 0.3137 0.8667] This is where functionality will be added to the different collectible types. Incredibly expansive and scalable.
  (if (== (`GameplayStatics.GetObjectClass` OtherActor) "/Game/Blueprints/FirstPersonCharacter.FirstPersonCharacter_C")
    (switch `/Game/Blueprints/KyleStuff/Enum_Collectibles` (`self.CollectibleType`))))

(fn `SetUp`
  (params (Mesh :type "StaticMesh Object Reference"))
  (`StaticMeshComponent.SetStaticMesh` (`self.CollectibleMesh`) Mesh))

(fn `UserConstructionScript`)