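; Item room pedestal that offers a random item from the Item_Room_Loot data table for the player to take.
; On BeginPlay it removes collected items from the row names, shuffles them, and displays the first pick's mesh.
; Overlap toggles input and a Gate, limiting Interact to a nearby player.
; Interacting applies the item's stats and destroys the pickup components, unless the Tome check passes and calls the HUD's UpgradedTome instead.
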(event `self.ReceiveBeginPlay`
  ;[1 0.3137 0.8667] Will decide which random item will be used on the stand. Need to set up the addition of stats and such.
  (bind _asfirst_person_character (cast `/Game/Blueprints/FirstPersonCharacter` (`GameplayStatics.GetPlayerPawn` 0)))
  (set `self.PlayerRef` _asfirst_person_character)
  (bind _outrownames (`DataTableFunctionLibrary.GetDataTableRowNames` "/Game/Blueprints/ItemRoom/Item_Room_Loot.Item_Room_Loot"))
  (bind _output_get (set `self.DataTableRows` _outrownames))
  (bind _returnvalue (`|GetDataTableRow` "/Game/Blueprints/ItemRoom/Item_Room_Loot.Item_Room_Loot" (`|GetArrayItem` (`self.RemoveFromItemPool` _output_get)))
    (:`then`
      (bind _output_get_2 (set `self.ChosenItem` _returnvalue))
      (`StaticMeshComponent.SetStaticMesh` (`self.StaticMesh`) (`.Mesh_20_C8D02B7D4B73145DCFC520AC2FBCB757` (break `/Game/Blueprints/ItemRoom/S_Items` _output_get_2))))))

(event `InputAction|Interact`
  (params (Key :type "Key Structure"))
  ;[1 0.3137 0.8667] Allows player interaction and stops enemies from messing with interaction.
  (:`Pressed`
    (`/Engine/EditorBlueprintResources/StandardMacros.Gate` true :!label _label
      (:`Exit`
        (if (== (`GameplayStatics.GetObjectClass` (`/Game/Blueprints/FirstPersonCharacter.EquippedGun` (`self.PlayerRef`))) "/Game/Blueprints/Weapons/BP_Tome.BP_Tome_C")
          (`/Game/Blueprints/Widgets/WBP_PlayerHUD.UpgradedTome` (`/Game/Blueprints/FirstPersonCharacter.HUDRef` (`self.PlayerRef`)))
          (else
            ;[1 0.3137 0.8667] Destroys collision to stop interaction and updates stats for player.
            (`ActorComponent.K2_DestroyComponent` (`self.Interact`))
            (`ActorComponent.K2_DestroyComponent` (`self.ItemMesh`))
            (set `self.Interactable` false)
            (`/Game/Blueprints/FirstPersonCharacter.UpdateStats` (`self.PlayerRef`) (`self.ChosenItem`))))))))

(event `self.Interact.OnComponentBeginOverlap`
  (params (OverlappedComponent :type "PrimitiveComponent Object Reference") (OtherActor :type "Actor Object Reference") (OtherComp :type "PrimitiveComponent Object Reference") (OtherBodyIndex :type Integer) (bFromSweep :type Boolean) (SweepResult :type "HitResult Structure (by ref)"))
  ;[1 0.3137 0.8667] Allows player interaction and stops enemies from messing with interaction.
  (if (and (== (`GameplayStatics.GetObjectClass` OtherActor) "/Game/Blueprints/FirstPersonCharacter.FirstPersonCharacter_C") (`self.Interactable`))
    (`self.EnableInput` (`GameplayStatics.GetPlayerController` 0))
    (goto _label :!via `Open`)))

(event `self.Interact.OnComponentEndOverlap`
  (params (OverlappedComponent :type "PrimitiveComponent Object Reference") (OtherActor :type "Actor Object Reference") (OtherComp :type "PrimitiveComponent Object Reference") (OtherBodyIndex :type Integer))
  ;[1 0.3137 0.8667] Allows player interaction and stops enemies from messing with interaction.
  (if (== (`GameplayStatics.GetObjectClass` OtherActor) "/Game/Blueprints/FirstPersonCharacter.FirstPersonCharacter_C")
    (`self.DisableInput` (`GameplayStatics.GetPlayerController` 0))
    (goto _label :!via `Close`)))

(fn `RemoveFromItemPool`
  (params (DataTableRows :type "Array of Name"))
  (returns (OptimisedItemPool :type "Array of Name"))
  (for _array_element (`/Game/Blueprints/FirstPersonCharacter.CollectedItems` (`self.PlayerRef`))
    (`KismetArrayLibrary.Array_RemoveItem` DataTableRows _array_element))
  (`KismetArrayLibrary.Array_Shuffle` DataTableRows)
  (return DataTableRows))

(fn `UserConstructionScript`)