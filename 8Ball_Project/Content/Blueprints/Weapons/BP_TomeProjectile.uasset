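; BP_TomeProjectile is the tome weapon's projectile, which explodes for area damage on overlapping anything except the player character or the tome.
; Detonate spawns a hit particle, then runs a stationary multi-sphere trace for pawns, ignoring the player.
; Each hit actor takes damage once, tracked in DamagedActors and scaled by the instigating player's DamageMultiplier, before the projectile destroys itself.
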(event `self.ReceiveBeginPlay`
  (set `self.PlayerRef` (cast `/Game/Blueprints/FirstPersonCharacter` (`self.Instigator`) :!pure true)))

(event `self.Sphere.OnComponentBeginOverlap`
  (params (OverlappedComponent :type "PrimitiveComponent Object Reference") (OtherActor :type "Actor Object Reference") (OtherComp :type "PrimitiveComponent Object Reference") (OtherBodyIndex :type Integer) (bFromSweep :type Boolean) (SweepResult :type "HitResult Structure (by ref)"))
  (if (not (or (== (`GameplayStatics.GetObjectClass` OtherActor) "/Game/Blueprints/FirstPersonCharacter.FirstPersonCharacter_C") (== (`GameplayStatics.GetObjectClass` OtherActor) "/Game/Blueprints/Weapons/BP_Tome.BP_Tome_C")))
    (`self.Detonate`)))

(fn `Detonate`
  (locals (DamagedActors :type "Array of Actor Object Reference"))
  (bind _returnvalue (`SceneComponent.K2_GetComponentLocation` (`self.DefaultSceneRoot`)))
  (`GameplayStatics.SpawnEmitterAtLocation` "/Game/AdvancedMagicFX12/particles/P_ky_hit.P_ky_hit" (`self.K2_GetActorLocation` self) (struct) (2.0 2.0 2.0))
  (bind _outhits (`KismetSystemLibrary.SphereTraceMultiForObjects` _returnvalue _returnvalue 400.0 (`|MakeArray` "ObjectTypeQuery3" :!type "EObjectTypeQuery Enum") false (`|MakeArray` (`GameplayStatics.GetPlayerCharacter` 0) :!type "Actor Object Reference") "None" true (struct :`R` 1.0 :`A` 1.0) (struct :`G` 1.0 :`A` 1.0) 2.0))
  (for _array_element _outhits
    (if (not (`KismetArrayLibrary.Array_Contains` (`local.DamagedActors`) (`.HitActor` (`GameplayStatics.BreakHitResult` _array_element))))
      (`GameplayStatics.ApplyDamage` (`.HitActor` (`GameplayStatics.BreakHitResult` _array_element)) (* (`/Game/Blueprints/FirstPersonCharacter.DamageMultiplier` (`self.PlayerRef`)) 100.0) (`GameplayStatics.GetPlayerController` 0) self)
      (`KismetArrayLibrary.Array_Add` (`local.DamagedActors`) (`.HitActor` (`GameplayStatics.BreakHitResult` _array_element)))))
  (`self.K2_DestroyActor`))

(fn `UserConstructionScript`)