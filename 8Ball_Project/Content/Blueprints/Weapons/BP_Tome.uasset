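; BP_Tome is a charge-based weapon that launches a BP_TomeProjectile for its Wielder.
; On BeginPlay it switches the Wielder's HUD ammo display to tome mode with an empty magazine.
; Fire requires the Wielder's TomeCharge to reach its maximum and CanFire to be true, then spawns the projectile at TomeFirePoint.
; Firing zeroes the charge stored on the Wielder, then calls AddTomeCharge with zero.
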(event `self.ReceiveBeginPlay`
  (`parent.ReceiveBeginPlay`)
  (`KismetSystemLibrary.PrintString` "Tome")
  (`/Game/Widgets/WBP_PlayerHUD.UpdateAmmo` (`/Game/Blueprints/FirstPersonCharacter.HUDRef` (`self.Wielder`)) true 0.0 0.0))

(event `/Game/Blueprints/Weapons/BPI_Weapon.Fire`
  (bind _wielder (`self.Wielder`))
  (bind _wielder_2 (`self.Wielder`))
  (bind _wielder_3 (`self.Wielder`))
  (bind _tomecharge (`/Game/Blueprints/FirstPersonCharacter.TomeCharge` _wielder_2))
  (`KismetSystemLibrary.PrintString` (`KismetStringLibrary.Conv_DoubleToString` _tomecharge))
  (if (>= _tomecharge (`/Game/Blueprints/FirstPersonCharacter.TomeChargeMax` _wielder_2))
    (if (`self.CanFire?`)
      (`KismetSystemLibrary.PrintString` "Tome fire")
      (`|SpawnActorFromClass` "/Game/Blueprints/Weapons/BP_TomeProjectile.BP_TomeProjectile_C" (`SceneComponent.K2_GetComponentToWorld` (`self.TomeFirePoint`)) "AlwaysSpawn" "OverrideRootScale" _wielder _wielder)
      (set `/Game/Blueprints/FirstPersonCharacter.TomeCharge` 0.0 _wielder_3)
      (`/Game/Blueprints/FirstPersonCharacter.AddTomeCharge` _wielder_3 0.0))))

(fn `UserConstructionScript`
  (`parent.UserConstructionScript`))