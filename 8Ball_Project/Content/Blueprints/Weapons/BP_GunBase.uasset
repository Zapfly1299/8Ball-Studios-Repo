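; BP_GunBase is a gun Blueprint that holds weapon stats and caches its wielding FirstPersonCharacter and GI_Main on BeginPlay.
; UpdateStats adds incoming stats, crossing MagSize and Range, while UpdateInstance and UpdateInstanceAmmo return rebuilt stat structs.
; Ammo functions push magazine counts to the wielder's HUD.
; SpawnHitEffect plays CurrentHitStruct's particle and sound at the hit location; its physical material is only printed, as surface selection is disconnected.
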(event `self.ReceiveBeginPlay`
  (bind _asfirst_person_character (cast `/Game/Blueprints/FirstPersonCharacter` (`self.Instigator`)))
  (set `self.Wielder` _asfirst_person_character)
  (`KismetSystemLibrary.PrintString` "GunBase beginplay fired")
  (bind _asgi_main (cast `/Game/Blueprints/KyleStuff/GI_Main` (`GameplayStatics.GetGameInstance`)))
  (set `self.InstanceRef` _asgi_main))

(fn `InitialAmmoSetup`
  (`/Game/Widgets/WBP_PlayerHUD.UpdateAmmo` (`/Game/Blueprints/FirstPersonCharacter.HUDRef` (`self.Wielder`)) false (`self.MagBullets`) (`self.MagSize`)))

(fn `SpawnHitEffect`
  (params (HitLocation :type "Vector Structure") (HitPhysMat :type "PhysicalMaterial Object Reference"))
  (bind (_currenthitstruct_hitparticle _currenthitstruct_hitsound) (break `/Game/Blueprints/HitStruct` (`self.CurrentHitStruct`)))
  (`KismetSystemLibrary.PrintString` (`KismetSystemLibrary.GetDisplayName` HitPhysMat))
  (`|ExecutionSequence`
    (:`then_0`
      (`GameplayStatics.SpawnEmitterAtLocation` _currenthitstruct_hitparticle HitLocation))
    (:`then_1`
      (`GameplayStatics.PlaySoundAtLocation` _currenthitstruct_hitsound HitLocation (struct) 1.0 1.0 0.0 null null null))))

(fn `Update Stats`
  (params (WeaponStats :type "/Game/Blueprints/Weapons/S_WeaponStats Structure"))
  (locals (`Tome?` :type Boolean))
  (bind (_firerate _damage _magsize _range _magbullets) (break `/Game/Blueprints/Weapons/S_WeaponStats` WeaponStats))
  (set `self.FireRate` (+ (`self.FireRate`) _firerate))
  (set `self.BaseDamage` (+ (`self.BaseDamage`) _damage))
  (set `self.BulletRange` (+ (`self.BulletRange`) _magsize))
  (set `self.MagSize` (+ (`self.MagSize`) _range))
  (set `self.MagBullets` _magbullets)
  (`/Game/Widgets/WBP_PlayerHUD.UpdateAmmo` (`/Game/Blueprints/FirstPersonCharacter.HUDRef` (`self.Wielder`)) false (`self.MagBullets`) (`self.MagSize`)))

(fn `UpdateInstance`
  (params (IncomingStats :type "/Game/Blueprints/Weapons/S_WeaponStats Structure") (InstanceStats :type "/Game/Blueprints/Weapons/S_WeaponStats Structure"))
  (returns (UpdatedStats :type "/Game/Blueprints/Weapons/S_WeaponStats Structure"))
  (bind (_firerate _damage _magsize _range) (break `/Game/Blueprints/Weapons/S_WeaponStats` InstanceStats))
  (bind (_firerate_2 _damage_2 _magsize_2 _range_2) (break `/Game/Blueprints/Weapons/S_WeaponStats` IncomingStats))
  ;[1 0.3137 0.8667] IF NO ONE LOOKS, IT'S STILL TIDY, RIGHT? YEAH? OKAY I THOUGHT SO AHAHAHAHAHHAHA
  (return (make `/Game/Blueprints/Weapons/S_WeaponStats` (+ _firerate _firerate_2) (+ _damage _damage_2) (+ _magsize _magsize_2) (+ _range _range_2))))

(fn `UpdateInstanceAmmo`
  (params (MagBullets :type "Float (double-precision)") (WeaponStats :type "/Game/Blueprints/Weapons/S_WeaponStats Structure"))
  (returns (Updated :type "/Game/Blueprints/Weapons/S_WeaponStats Structure"))
  (locals (UpdatedWeapon :type "/Game/Blueprints/Weapons/S_WeaponStats Structure"))
  (bind (_firerate _damage _magsize _range) (break `/Game/Blueprints/Weapons/S_WeaponStats` WeaponStats))
  (`/Game/Widgets/WBP_PlayerHUD.UpdateAmmo` (`/Game/Blueprints/FirstPersonCharacter.HUDRef` (`self.Wielder`)) false MagBullets (`self.MagSize`))
  (bind _output_get (set `local.UpdatedWeapon` (make `/Game/Blueprints/Weapons/S_WeaponStats` _firerate _damage _magsize _range MagBullets)))
  (return _output_get))

(fn `UserConstructionScript`)