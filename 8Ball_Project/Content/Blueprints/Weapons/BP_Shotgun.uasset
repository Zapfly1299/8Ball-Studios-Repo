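; Shotgun weapon Blueprint that loads its stats from the instance reference and saves ammo changes back to it.
; Fire casts scattered camera line traces per pellet, spawning hit effects and applying damage scaled by a distance-sampled falloff timeline and the wielder's multiplier.
; A delay gates fire rate, and an empty magazine triggers a timeline that pitches the gun mesh before refilling.
; IncreaseStats saves upgrades to the TommyGun entry, not Shotgun.
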(event `/Game/Blueprints/Weapons/BPI_Weapon.AmmoRecheck`
  (`/Game/Widgets/WBP_PlayerHUD.UpdateAmmo` (`/Game/Blueprints/FirstPersonCharacter.HUDRef` (`self.Wielder`)) false (`self.MagBullets`) (`self.MagSize`)))

(event `self.ReceiveBeginPlay`
  (`parent.ReceiveBeginPlay`)
  (`KismetSystemLibrary.PrintString` "shotgun")
  ;[1 0.3137 0.8667] Makes sure stats are carried over when actor is spawned
  (`self.Update Stats` (`/Game/Blueprints/KyleStuff/GI_Main.Shotgun` (`self.InstanceRef`))))

(event `/Game/Blueprints/Weapons/BPI_Weapon.IncreaseStats`
  (params (Stats :type "/Game/Blueprints/Weapons/S_WeaponStats Structure"))
  ;[1 0.3137 0.8667] Increases the stats of the weapon and saves the increases to instance
  (bind _output_get (set `self.IncomingStats` Stats))
  (`self.Update Stats` _output_get)
  (bind _updatedstats (`self.UpdateInstance` (`self.IncomingStats`) (`/Game/Blueprints/KyleStuff/GI_Main.Tommy Gun` (`self.InstanceRef`))))
  (set `/Game/Blueprints/KyleStuff/GI_Main.Tommy Gun` _updatedstats (`self.InstanceRef`)))

(event `/Game/Blueprints/Weapons/BPI_Weapon.Fire`
  (bind _returnvalue (* 0.0 -1.0))
  (bind _instanceref (`self.InstanceRef`))
  (bind _instanceref_2 (`self.InstanceRef`))
  (bind _firstpersoncamera (`/Game/Blueprints/FirstPersonCharacter.FirstPersonCamera` (`self.Wielder`)))
  (bind _returnvalue_2 (`SceneComponent.K2_GetComponentLocation` _firstpersoncamera))
  (bind (_returnvalue_x _returnvalue_y _returnvalue_z) (`KismetMathLibrary.BreakVector` (+ _returnvalue_2 (* (`SceneComponent.GetForwardVector` _firstpersoncamera) (`self.BulletRange`)))))
  (if (`self.CanFire?`)
    (if (> (`self.MagBullets`) 0.0)
      (`KismetSystemLibrary.PrintString` "shotgun fire")
      ;[1 1 1] Fire FX
      (`self.FireEffect`)
      (for _ (range 1 (+ (`self.PelletAmount`) 1))
        ;[1 1 1] Linetrace
        (bind (_outhit _returnvalue_3) (`KismetSystemLibrary.LineTraceSingleForObjects` _returnvalue_2 (`KismetMathLibrary.MakeVector` (+ _returnvalue_x (`KismetMathLibrary.RandomFloatInRange` _returnvalue 0.0)) (+ _returnvalue_y (`KismetMathLibrary.RandomFloatInRange` _returnvalue 0.0)) (+ _returnvalue_z (`KismetMathLibrary.RandomFloatInRange` _returnvalue 0.0))) (`|MakeArray` "ObjectTypeQuery1" "ObjectTypeQuery2" "ObjectTypeQuery3" "ObjectTypeQuery4" "ObjectTypeQuery6" :!type "EObjectTypeQuery Enum") false (`|MakeArray` self (`GameplayStatics.GetPlayerCharacter` 0) :!type "Actor Object Reference") "Persistent"))
        (if _returnvalue_3
          ;[1 1 1] Hit FX
          (`self.SpawnHitEffect` (`.Location` (`GameplayStatics.BreakHitResult` _outhit)) (`.PhysMat` (`GameplayStatics.BreakHitResult` _outhit)))
          (`|ExecutionSequence`
            (:`then_0`
              ;[1 1 1] Calculate range dropoff
              (bind (_direction _newtrack_0) (`Timeline|RangeDropoff` :`NewTime` (`KismetMathLibrary.Vector_Distance` (`.Location` (`GameplayStatics.BreakHitResult` _outhit)) (`self.K2_GetActorLocation` self)) :!via `SetNewTime`)))
            (:`then_1`
              ;[1 1 1] Apply Damage
              (`GameplayStatics.ApplyDamage` (`.HitActor` (`GameplayStatics.BreakHitResult` _outhit)) (* _newtrack_0 (* (`self.BaseDamage`) (`/Game/Blueprints/FirstPersonCharacter.DamageMultiplier` (`self.Wielder`)))) (`GameplayStatics.GetPlayerController` 0) self)))))
      (set `self.CanFire?` false)
      (bind _output_get (set `self.MagBullets` (- (`self.MagBullets`) 1.0)))
      (set `/Game/Blueprints/KyleStuff/GI_Main.Shotgun` (`self.UpdateInstanceAmmo` _output_get (`/Game/Blueprints/KyleStuff/GI_Main.Shotgun` _instanceref_2)) _instanceref_2)
      (if (> _output_get 0.0)
        ;[1 1 1] Firerate
        (`KismetSystemLibrary.Delay` (`self.FireRate`))
        (set `self.CanFire?` true)
        (else
          (bind (_direction_2 _newtrack_0_2) (`Timeline|ReloadTimeline` :!via `PlayFromStart` :!label _label)
            (:`Update`
              (`SceneComponent.K2_SetRelativeRotation` (`self.GunMesh`) (`KismetMathLibrary.MakeRotator` 0.0 _newtrack_0_2) false false))
            (:`Finished`
              (bind _output_get_2 (set `self.MagBullets` (`self.MagSize`)))
              (set `/Game/Blueprints/KyleStuff/GI_Main.Shotgun` (`self.UpdateInstanceAmmo` _output_get_2 (`/Game/Blueprints/KyleStuff/GI_Main.Shotgun` _instanceref)) _instanceref)
              (set `self.CanFire?` true)
              (set `self.IsReloading` false)))))
      (else
        (`/Game/Blueprints/Weapons/BPI_Weapon.Reload`)))))

(event `/Game/Blueprints/Weapons/BPI_Weapon.Reload`
  (set `self.CanFire?` false)
  (set `self.IsReloading` true)
  (goto _label :!via `PlayFromStart`))

(fn `FireEffect`
  (bind _firepoint (`self.FirePoint`))
  (bind (_returnvalue_location _returnvalue_rotation) (`KismetMathLibrary.BreakTransform` (`SceneComponent.K2_GetComponentToWorld` _firepoint)))
  (`GameplayStatics.SpawnEmitterAttached` "/Game/StarterContent/Particles/P_Explosion.P_Explosion" _firepoint "None" _returnvalue_location _returnvalue_rotation (0.3 0.3 0.3) "KeepWorldPosition")
  (`GameplayStatics.PlaySoundAtLocation` "/Game/Blueprints/Audio+Effects/Winchester12-RA_The_Sun_God-1722751268.Winchester12-RA_The_Sun_God-1722751268" _returnvalue_location (struct) 1.0 1.0 0.0 null null null))

(fn `UserConstructionScript`
  (`parent.UserConstructionScript`))