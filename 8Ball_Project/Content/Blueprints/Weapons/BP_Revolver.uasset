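; BP_Revolver is a hitscan weapon that fires from the wielder's first-person camera, with double damage on "Headshot"-tagged components.
; Fire plays effects, applies multiplied damage, gates shots by fire rate, and drives timeline-based camera recoil and gun kick.
; An empty magazine triggers an automatic reload, animated by rolling the gun mesh on a timeline.
; Stats and ammo are saved to InstanceRef and restored on spawn, so upgrades carry over.
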(event `self.AmmoRecheck`
  (`/Game/Widgets/WBP_PlayerHUD.UpdateAmmo` (`/Game/Blueprints/FirstPersonCharacter.HUDRef` (`self.Wielder`)) false (`self.MagBullets`) (`self.MagSize`)))

(event `self.ReceiveBeginPlay`
  (`parent.ReceiveBeginPlay`)
  (`KismetSystemLibrary.PrintString` "revolver")
  ;[1 0.3137 0.8667] Makes sure stats are carried over when actor is spawned
  (`self.Update Stats` (`/Game/Blueprints/KyleStuff/GI_Main.Revolver` (`self.InstanceRef`))))

(event `self.IncreaseStats`
  (params (Stats :type "/Game/Blueprints/Weapons/S_WeaponStats Structure"))
  ;[1 0.3137 0.8667] Increases the stats of the weapon and saves the increases to instance
  (bind _output_get (set `self.IncomingStats` Stats))
  (`self.Update Stats` _output_get)
  (bind _updatedstats (`self.UpdateInstance` (`self.IncomingStats`) (`/Game/Blueprints/KyleStuff/GI_Main.Revolver` (`self.InstanceRef`))))
  (set `/Game/Blueprints/KyleStuff/GI_Main.Revolver` _updatedstats (`self.InstanceRef`)))

(event `self.Fire`
  (bind _returnvalue (`GameplayStatics.GetPlayerController` 0))
  (bind _wielder (`self.Wielder`))
  (bind _instanceref (`self.InstanceRef`))
  (bind (_returnvalue_location _returnvalue_rotation) (`KismetMathLibrary.BreakTransform` (`SceneComponent.GetRelativeTransform` (`self.GunMesh`))))
  (bind _firstpersoncamera (`/Game/Blueprints/FirstPersonCharacter.FirstPersonCamera` (`self.Wielder`)))
  (bind _returnvalue_2 (`SceneComponent.K2_GetComponentLocation` _firstpersoncamera))
  (bind _returnvalue_3 (* (`self.BaseDamage`) (`/Game/Blueprints/FirstPersonCharacter.DamageMultiplier` (`self.Wielder`))))
  ;[1 1 1] Firing
  (if (`self.CanFire?`)
    (if (> (`self.MagBullets`) 0.0)
      (`KismetSystemLibrary.PrintString` "revolver fire")
      (`|ExecutionSequence`
        (:`then_0`
          ;;[1 1 1] Fire FX
          (`self.FireEffects`)
          ;;[1 1 1] Linetrace
          (bind (_outhit _returnvalue_4) (`KismetSystemLibrary.LineTraceSingleForObjects` _returnvalue_2 (+ _returnvalue_2 (* (`SceneComponent.GetForwardVector` _firstpersoncamera) (`self.BulletRange`))) (`|MakeArray` "ObjectTypeQuery3" "ObjectTypeQuery6" "ObjectTypeQuery1" :!type "EObjectTypeQuery Enum") false (`|MakeArray` self (`GameplayStatics.GetPlayerCharacter` 0) :!type "Actor Object Reference")))
          (`|ExecutionSequence`
            (:`then_0`
              (if _returnvalue_4
                ;;[1 1 1] Hit FX
                (`self.SpawnHitEffect` (`.Location` (`GameplayStatics.BreakHitResult` _outhit)) (`.PhysMat` (`GameplayStatics.BreakHitResult` _outhit)))
                ;;[1 1 1] Apply Damage
                (if (`ActorComponent.ComponentHasTag` (`.HitComponent` (`GameplayStatics.BreakHitResult` _outhit)) "Headshot")
                  (`GameplayStatics.ApplyDamage` (`.HitActor` (`GameplayStatics.BreakHitResult` _outhit)) (* _returnvalue_3 2.0) _returnvalue self)
                  (`KismetSystemLibrary.PrintString` "headshot!")
                  (else
                    (`KismetSystemLibrary.PrintString` (`KismetSystemLibrary.GetDisplayName` (`.HitComponent` (`GameplayStatics.BreakHitResult` _outhit))))
                    (`GameplayStatics.ApplyDamage` (`.HitActor` (`GameplayStatics.BreakHitResult` _outhit)) _returnvalue_3 _returnvalue self))))
              (set `self.CanFire?` false)
              (bind _output_get (set `self.MagBullets` (- (`self.MagBullets`) 1.0)))
              (set `/Game/Blueprints/KyleStuff/GI_Main.Revolver` (`self.UpdateInstanceAmmo` _output_get (`/Game/Blueprints/KyleStuff/GI_Main.Revolver` _instanceref)) _instanceref)
              (if (> _output_get 0.0)
                ;;[1 1 1] Fire rate stuff
                (`KismetSystemLibrary.Delay` (`self.FireRate`))
                (if (not (`self.IsReloading`))
                  (set `self.CanFire?` true))
                (else
                  (`self.Reload`))))
            (:`then_1`
              (set `self.RecoilYaw+-` (`KismetMathLibrary.RandomIntegerInRange` -1 1))
              (`Timeline|RecoilTimeline` :!via `PlayFromStart`
                (:`Update`
                  (`Pawn.AddControllerPitchInput` _wielder (`KismetMathLibrary.RandomFloatInRange` -0.15 -0.2))
                  (`Pawn.AddControllerYawInput` _wielder (* (`self.RecoilYaw+-`) (`KismetMathLibrary.RandomFloatInRange` 0.1 0.2))))))))
        (:`then_1`
          ;;[1 1 1] Play RevolverClick
          (`KismetSystemLibrary.Delay` (- (`self.FireRate`) 0.15))
          (`GameplayStatics.PlaySoundAtLocation` "/Game/Blueprints/Audio+Effects/Revolver/RevolverClick.RevolverClick" (`SceneComponent.K2_GetComponentLocation` (`self.GunMesh`)) (struct) 1.0 1.0 0.0 null null null))
        (:`then_2`
          ;[1 1 1] Recoil Anim
          (set `self.StartRecoilLoc` _returnvalue_location)
          (set `self.StartRecoilRot` _returnvalue_rotation)
          (bind (_direction _track1) (`Timeline|RecoilAnim` :!via `PlayFromStart`)
            (:`Update`
              (`SceneComponent.K2_SetRelativeLocationAndRotation` (`self.GunMesh`) (+ (`KismetMathLibrary.MakeVector` (.x _track1) 0.0 (.y _track1)) (`self.StartRecoilLoc`)) (`KismetMathLibrary.ComposeRotators` (`self.StartRecoilRot`) (`KismetMathLibrary.MakeRotator` 0.0 (.z _track1))) false false)))))
      (else
        (`self.Reload`)))))

(event `self.Reload`
  (bind _instanceref (`self.InstanceRef`))
  ;[1 1 1] Firing
  (set `self.CanFire?` false)
  (set `self.IsReloading` true)
  ;;[1 1 1] Reload
  (bind (_direction _newtrack_0) (`Timeline|ReloadTimeline` :!via `PlayFromStart`)
    (:`Update`
      (`SceneComponent.K2_SetRelativeRotation` (`self.GunMesh`) (`KismetMathLibrary.MakeRotator` _newtrack_0 0.0 270.0) false false))
    (:`Finished`
      (bind _output_get (set `self.MagBullets` (`self.MagSize`)))
      (set `/Game/Blueprints/KyleStuff/GI_Main.Revolver` (`self.UpdateInstanceAmmo` _output_get (`/Game/Blueprints/KyleStuff/GI_Main.Revolver` _instanceref)) _instanceref)
      (set `self.CanFire?` true)
      (set `self.IsReloading` false))))

(fn `FireEffects`
  (bind _firepoint (`self.FirePoint`))
  (bind (_returnvalue_location _returnvalue_rotation) (`KismetMathLibrary.BreakTransform` (`SceneComponent.K2_GetComponentToWorld` _firepoint)))
  (`GameplayStatics.SpawnEmitterAttached` "/Game/StarterContent/Particles/P_Explosion.P_Explosion" _firepoint "None" _returnvalue_location _returnvalue_rotation (0.1 0.1 0.1) "KeepWorldPosition")
  (`GameplayStatics.PlaySoundAtLocation` "/Game/Blueprints/Audio+Effects/Revolver/Cue_RevolverShotRev.Cue_RevolverShotRev" _returnvalue_location (struct) 1.0 1.0 0.0 null null null))

(fn `UserConstructionScript`
  (`parent.UserConstructionScript`))