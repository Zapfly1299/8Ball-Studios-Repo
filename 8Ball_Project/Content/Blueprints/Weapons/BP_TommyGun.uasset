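; Tommy gun weapon Blueprint for automatic fire, driven by a looping timer that runs until stopped or reloading.
; Each shot line traces from the wielder's camera with random spread and persistent debug drawing, applying multiplier-scaled damage and hit effects.
; An empty magazine triggers a timeline reload that pitches the mesh, then refills ammo.
; Stats and ammo are saved to InstanceRef, with stats restored on BeginPlay.
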(event `self.AmmoRecheck`
  (`/Game/Widgets/WBP_PlayerHUD.UpdateAmmo` (`/Game/Blueprints/FirstPersonCharacter.HUDRef` (`self.Wielder`)) false (`self.MagBullets`) (`self.MagSize`)))

(event `self.ReceiveBeginPlay`
  ;[0.2044 0.3892 1] BEGINPLAY
  (`parent.ReceiveBeginPlay`)
  (`KismetSystemLibrary.PrintString` "tommygun")
  ;[1 0.3137 0.8667] Makes sure stats are carried over when actor is spawned
  (`self.Update Stats` (`/Game/Blueprints/KyleStuff/GI_Main.Tommy Gun` (`self.InstanceRef`))))

(event `self.StopFiring`
  ;[0.2044 0.3892 1] Start and stop shooting
  (`KismetSystemLibrary.K2_ClearAndInvalidateTimerHandle` (stale `self.Fire` _returnvalue)))

(event `self.Fire`
  ;[0.2044 0.3892 1] Start and stop shooting
  (if (and (`self.CanFire?`) (not (`self.IsReloading`)))
    (if (> (`self.MagBullets`) 0.0)
      (bind _returnvalue (`KismetSystemLibrary.K2_SetTimer` null "Shooting" 0.1 true))
      (else
        (`self.Reload`)))))

(event `self.IncreaseStats`
  (params (Stats :type "/Game/Blueprints/Weapons/S_WeaponStats Structure"))
  ;[1 0.3137 0.8667] Increases the stats of the weapon and saves the increases to instance
  (bind _output_get (set `self.IncomingStats` Stats))
  (`self.Update Stats` _output_get)
  (bind _updatedstats (`self.UpdateInstance` (`self.IncomingStats`) (`/Game/Blueprints/KyleStuff/GI_Main.Tommy Gun` (`self.InstanceRef`))))
  (set `/Game/Blueprints/KyleStuff/GI_Main.Tommy Gun` _updatedstats (`self.InstanceRef`)))

(event `Shooting`
  (bind _instanceref (`self.InstanceRef`))
  (bind _firstpersoncamera (`/Game/Blueprints/FirstPersonCharacter.FirstPersonCamera` (`self.Wielder`)))
  (bind _returnvalue (`SceneComponent.K2_GetComponentLocation` _firstpersoncamera))
  (bind (_returnvalue_x _returnvalue_y _returnvalue_z) (`KismetMathLibrary.BreakVector` (+ _returnvalue (* (`SceneComponent.GetForwardVector` _firstpersoncamera) (`self.BulletRange`)))))
  ;[0.2044 0.3892 1] Shooting
  (`self.FireEffects`)
  (`|ExecutionSequence`
    (:`then_0`
      (bind (_outhit _returnvalue_2) (`KismetSystemLibrary.LineTraceSingleForObjects` _returnvalue (`KismetMathLibrary.MakeVector` (+ _returnvalue_x (`KismetMathLibrary.RandomFloatInRange` -150.0 150.0)) (+ _returnvalue_y (`KismetMathLibrary.RandomFloatInRange` -150.0 150.0)) (+ _returnvalue_z (`KismetMathLibrary.RandomFloatInRange` -150.0 150.0))) (`|MakeArray` "ObjectTypeQuery1" "ObjectTypeQuery2" "ObjectTypeQuery3" "ObjectTypeQuery4" "ObjectTypeQuery6" :!type "EObjectTypeQuery Enum") false (`|MakeArray` self (`GameplayStatics.GetPlayerCharacter` 0) :!type "Actor Object Reference") "Persistent"))
      (if _returnvalue_2
        (`self.SpawnHitEffect` (`.Location` (`GameplayStatics.BreakHitResult` _outhit)) (`.PhysMat` (`GameplayStatics.BreakHitResult` _outhit)))
        (`GameplayStatics.ApplyDamage` (`.HitActor` (`GameplayStatics.BreakHitResult` _outhit)) (* (`self.BaseDamage`) (`/Game/Blueprints/FirstPersonCharacter.DamageMultiplier` (`self.Wielder`))) (`GameplayStatics.GetPlayerController` 0) self)))
    (:`then_1`
      (bind _output_get (set `self.MagBullets` (- (`self.MagBullets`) 1.0)))
      (set `/Game/Blueprints/KyleStuff/GI_Main.Tommy Gun` (`self.UpdateInstanceAmmo` _output_get (`/Game/Blueprints/KyleStuff/GI_Main.Tommy Gun` _instanceref)) _instanceref)
      (if (not (> _output_get 0.0))
        (`self.Reload`)))))

(event `self.Reload`
  (bind _instanceref (`self.InstanceRef`))
  ;[0.2044 0.3892 1] Shooting
  (set `self.IsReloading` true)
  (set `self.CanFire?` false)
  (`self.StopFiring`)
  (bind (_direction _newtrack_0) (`Timeline|ReloadTimeline` :!via `PlayFromStart`)
    (:`Update`
      (`SceneComponent.K2_SetRelativeRotation` (`self.GunMesh`) (`KismetMathLibrary.MakeRotator` 0.0 _newtrack_0) false false))
    (:`Finished`
      (bind _output_get (set `self.MagBullets` (`self.MagSize`)))
      (set `/Game/Blueprints/KyleStuff/GI_Main.Tommy Gun` (`self.UpdateInstanceAmmo` _output_get (`/Game/Blueprints/KyleStuff/GI_Main.Tommy Gun` _instanceref)) _instanceref)
      (set `self.CanFire?` true)
      (set `self.IsReloading` false))))

(fn `FireEffects`
  (bind _firepoint (`self.FirePoint`))
  (bind (_returnvalue_location _returnvalue_rotation) (`KismetMathLibrary.BreakTransform` (`SceneComponent.K2_GetComponentToWorld` _firepoint)))
  (`GameplayStatics.SpawnEmitterAttached` "/Game/StarterContent/Particles/P_Explosion.P_Explosion" _firepoint "None" _returnvalue_location _returnvalue_rotation (0.1 0.1 0.1) "KeepWorldPosition")
  (`GameplayStatics.PlaySoundAtLocation` "/Game/Blueprints/Audio+Effects/RevolverShot.RevolverShot" _returnvalue_location (struct) 1.0 1.0 0.0 null null null))

(fn `UserConstructionScript`
  (`parent.UserConstructionScript`))